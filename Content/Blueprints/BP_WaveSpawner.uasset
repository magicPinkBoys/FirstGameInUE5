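; BP_WaveSpawner is an actor that runs successive waves of BP_Enermy enemies, starting the first on BeginPlay.
; SpawnWave increments CurrentWave, takes that wave's enemy count from the values of the Waves map, and spawns them at its own transform.
; CheckforEnermies, which nothing in this graph calls, waits briefly and starts the next wave when no enemies remain.
; The wave index has no bounds check.
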(event Custom|Spawn%20Wave
  ;[0.224 0.224 0.224] Spwan
  (Math|Integer|IncrementInt (Variables|Default|GetCurrent%20Wave)
    (:%20%20
      (bind _values (Utilities|Map|Values (Variables|Default|GetWaves)))
      (for _index (range 1 (Utilities|Array|Get(acopy) _values (- (Variables|Default|GetCurrent%20Wave) 1)))
        (Game|SpawnActorfromClass "/Game/Blueprints/BP_Enermy.BP_Enermy_C" (Transformation|GetActorTransform) "AdjustIfPossibleButAlwaysSpawn" "MultiplyWithRoot" 0 0)))))

(event Custom|Check%20for%20Enermies
  ;[0.224 0.224 0.224] Spawn Next Level
  (Utilities|FlowControl|Delay 0.2)
  (bind _outactors (Actor|GetAllActorsOfClass "/Game/Blueprints/BP_Enermy.BP_Enermy_C"))
  (if (== (Utilities|Array|Length _outactors) 0)
    (CallFunction|SpawnWave)))

(event EventBeginPlay
  ;[0.224 0.224 0.224] Start
  (CallFunction|SpawnWave))

(fn ConstructionScript)